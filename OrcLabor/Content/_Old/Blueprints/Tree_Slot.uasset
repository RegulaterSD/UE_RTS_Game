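; Clickable tree actor that yields wood once to the RTS resource economy.
; BeginPlay enables click and mouse-over events on the first player controller.
; The first click hides the tree's static mesh and cube, adds WoodGiven through the RTS_Resource_Manager found by class lookup, and sets Harvested.
; Later clicks only print a debug message that the tree is already harvested.
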(event EventBeginPlay
  (bind _returnvalue (Game|GetPlayerController 0))
  ;[1 1 1] Set up events
  (Variables|/Script/Engine.PlayerController|SetbEnableClickEvents _returnvalue true)
  (Variables|/Script/Engine.PlayerController|SetbEnableMouseOverEvents _returnvalue true))

(event MouseInput|EventActorOnClicked
  (params (ButtonPressed :type Key%20Structure :default "None"))
  ;[1 1 1] On Click
  (Development|PrintString "Clicked on  Tree")
  (if (Variables|Default|GetHarvested)
    (Development|PrintString "Tree Already harvested")
    (else
      (Development|PrintString "Tree harvested")
      (Rendering|ToggleVisibility (Variables|Default|GetStaticMesh) false)
      (Rendering|ToggleVisibility (Variables|Default|GetCube) false)
      (bind _returnvalue (Actor|GetActorOfClass "/Game/TopDown/Blueprints/Resources/RTS_Resource_Manager.RTS_Resource_Manager_C"))
      (Default|AddWood _returnvalue (Variables|Default|GetWood%20Given))
      (Variables|Default|SetHarvested true))))

(fn ConstructionScript)