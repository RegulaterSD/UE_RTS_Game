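; RTS_Sound_Manager is an unfinished actor meant to switch background audio based on whether enemy units are present.
; Every tick it gathers actors tagged EnemyUnit and sets IsEnemyOnMap to true when none are found, inverse to the variable's name.
; The branch choosing between the forest day and action sounds is disconnected, so nothing plays.
; GrabSelectedUnits and the other events are empty stubs.
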(event Custom|CustomEvent)

(event EventBeginPlay)

(event EventTick
  (params (DeltaSeconds :type Float%20%28single-precision%29))
  (bind _outactors (Actor|GetAllActorswithTag "EnemyUnit"))
  (Variables|Default|SetOut%20ActorsTag _outactors)
  (bind _output_get (Variables|Default|SetIsEnemyOnMap (== (Utilities|Array|Length (Variables|Default|GetOut%20ActorsTag)) 0)))
  (if _output_get
    _))

(fn ConstructionScript)

(fn GrabSelectedUnits
  (return 0))