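; HUD class for RTS marquee selection of player units, driven by press, hold and release events that track mouse positions.
; While dragging, DrawHUD draws a translucent rectangle and, inside a loop over Player_Tower actors, gathers Player_Unit actors within it.
; It messages units to select up to a limit, clears building selection, and deselects units outside the rectangle.
; Separate events select one unit or clear all, and GrabSelectedUnits exposes the selection.
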(event EventClearSelectedUnits
  (bind _selectedunits (Variables|Default|GetSelectedUnits))
  ;[1 1 1] Clear Selected Units
  (for _array_element _selectedunits
    (Class|RTSInterface|DeselectThis(Message) _array_element))
  (Utilities|Array|Clear _selectedunits))

(event EventSelectSingleUnit
  (params (Unit :type Actor%20Object%20Reference))
  ;[1 1 1] Select Single Unit
  (Class|RTSInterface|SelectThis(Message) Unit)
  (Utilities|Array|AddUnique (Variables|Default|GetSelectedUnits) Unit))

(event EventMarqueePressed
  (bind _returnvalue (Game|GetPlayerController 0))
  (bind (_locationx _locationy) (Game|Player|GetMousePosition _returnvalue))
  ;[1 1 1] Marquee Start
  (Variables|Default|SetIsDrawing true)
  (bind _output_get (Variables|Default|SetStartMousePosition (Math|Vector2D|MakeVector2D _locationx _locationy)))
  (Variables|Default|SetCurrentMousePostion _output_get))

(event EventMarqueeHeld
  (bind _returnvalue (Game|GetPlayerController 0))
  (bind (_locationx _locationy) (Game|Player|GetMousePosition _returnvalue))
  ;[1 1 1] Marquee Held
  (Variables|Default|SetCurrentMousePostion (Math|Vector2D|MakeVector2D _locationx _locationy)))

(event EventMarqueeReleased
  ;[1 1 1] Marquee Released
  (Variables|Default|SetIsDrawing false))

(event EventDrawHUD
  (params (SizeX :type Integer) (SizeY :type Integer))
  (bind _startmouseposition (Variables|Default|GetStartMousePosition))
  (bind _currentmousepostion (Variables|Default|GetCurrentMousePostion))
  (bind _selectedunits (Variables|Default|GetSelectedUnits))
  (bind _startmouseposition_2 (Variables|Default|GetStartMousePosition))
  (bind _currentmousepostion_2 (Variables|Default|GetCurrentMousePostion))
  (bind _outactors (Class|HUD|GetActorsinSelectionRectangle "/Game/OrcLaborContent/Blueprints/Units/Player_Unit.Player_Unit_C" _startmouseposition _currentmousepostion false false))
  ;[1 1 1] Marquee Drag Select Array
  ;;[0.3325 0.3325 0.3325] Draw Rect
  (if (Variables|Default|GetIsDrawing)
    (HUD|DrawRect "(R=0.527115,G=0.527115,B=0.527115,A=0.200000)" (.x _startmouseposition_2) (.y _startmouseposition_2) (- (.x _currentmousepostion_2) (.x _startmouseposition_2)) (- (.y _currentmousepostion_2) (.y _startmouseposition_2)))
    ;;[0.3325 0.3325 0.3325] Get Player Actors Under Rect
    (Actor|GetAllActorsOfClass "/Game/OrcLaborContent/Blueprints/Units/Player_Tower.Player_Tower_C")
    (for _array_element 0
      (Utilities|Array|RemoveItem _outactors _array_element)
      (bind _output_get (Variables|Default|SetActorsInRect _outactors))
      ;;[0.3325 0.3325 0.3325] Select Units
      (for _array_element_2 _output_get
        ;;;[1 1 1] Limit Unit Selection
        (if (not (>= (Utilities|Array|Length _selectedunits) (Variables|Default|GetUnitSelectionLimit)))
          (Class|RTSInterface|SelectThis(Message) _array_element_2)
          (Utilities|Array|AddUnique _selectedunits _array_element_2)
          (Class|RTSInterface|ClearSelectedBuilding(Message) (Game|GetPlayerController 0))))
      ;;[0.3325 0.3325 0.3325] Deselect Units
      (for _array_element_3 (Variables|Default|GetSelectedUnits)
        (if (== (Utilities|Array|FindItem (Variables|Default|GetActorsInRect) _array_element_3) -1)
          (Class|RTSInterface|DeselectThis(Message) _array_element_3)
          (Utilities|Array|RemoveItem (Variables|Default|GetSelectedUnits) _array_element_3))))))

(fn ConstructionScript)

(fn GrabSelectedUnits
  (return (Variables|Default|GetSelectedUnits)))