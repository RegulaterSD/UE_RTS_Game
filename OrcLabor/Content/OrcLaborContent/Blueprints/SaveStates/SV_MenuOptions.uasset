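; SV_MenuOptions is a save game object that stores master, music and SFX volume settings for the options menu.
; Two identical save events call LoadSettings, write the three volumes into the resulting object and save it to the "sv_options" slot.
; LoadSettings loads that slot or creates a new instance, so the object writes through a reference to another instance of its own class.
; GrabSelectedUnits is an empty stub.
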(event Custom|Save%20Menu%20Settings
  (params (MasterVolume :type Float%20%28double-precision%29) (MusicVolume :type Float%20%28double-precision%29) (SFXVolume :type Float%20%28double-precision%29))
  (bind _sv_menu_options (Variables|Default|GetSV%20Menu%20Options))
  (Utilities|LoadSettings)
  (Variables|SV_MenuOptions_C|SetMaster%20Volume _sv_menu_options (stale EventSaveMenuOptions Master%20Volume))
  (Variables|SV_MenuOptions_C|SetMusic%20Volume _sv_menu_options (stale EventSaveMenuOptions Music%20Volume))
  (Variables|SV_MenuOptions_C|SetSFX%20Volume _sv_menu_options (stale EventSaveMenuOptions SFX%20Volume))
  (SaveGame|SaveGametoSlot (Variables|Default|GetSV%20Menu%20Options) "sv_options"))

(event EventSaveMenuOptions
  (params (Master%20Volume :type Float%20%28double-precision%29) (Music%20Volume :type Float%20%28double-precision%29) (SFX%20Volume :type Float%20%28double-precision%29))
  (bind _sv_menu_options (Variables|Default|GetSV%20Menu%20Options))
  (Utilities|LoadSettings)
  (Variables|SV_MenuOptions_C|SetMaster%20Volume _sv_menu_options Master%20Volume)
  (Variables|SV_MenuOptions_C|SetMusic%20Volume _sv_menu_options Music%20Volume)
  (Variables|SV_MenuOptions_C|SetSFX%20Volume _sv_menu_options SFX%20Volume)
  (SaveGame|SaveGametoSlot (Variables|Default|GetSV%20Menu%20Options) "sv_options"))

(fn GrabSelectedUnits
  (return 0))