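; AI controller for RTS tower units that runs RTS_TowerBT and picks the enemy to attack.
; Sensed actors tagged EnemyUnit become the blackboard attack target only if the current one is missing or dead.
; Perception is wiped after each such evaluation, and dead actors are rejected through an IsDead message.
; ClickToAttack overrides the target with any living actor, while GrabSelectedUnits is an empty stub.
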(event OnTargetPerceptionUpdated(AIPerception)
  (params (Actor :type Actor%20Object%20Reference) (Stimulus :type AI%20Stimulus%20Structure))
  ;[1 1 1] AI Perception
  (if (Actor|ActorHasTag Actor "EnemyUnit")
    (if (.bSuccessfullySensed (Utilities|Struct|BreakAIStimulus Stimulus))
      (bind _isdead (Class|RTSIBPDamageable|IsDead(Message) Actor))
      (if _isdead
        (Class|AIPerceptionComponent|ForgetAll (Variables|Default|GetAIPerception))
        (else
          (CallFunction|FollowNewEnemyTarget Actor))))))

(event EventBeginPlay
  ;[1 1 1] Run Behavior Tree
  (AI|RunBehaviorTree "/Game/OrcLaborContent/Blueprints/Unit_AI/RTS_TowerBT.RTS_TowerBT"))

(fn ConstructionScript)

(fn FollowNewEnemyTarget
  (params (TargetToFollow :type Object%20Object%20Reference))
  (bind _returnvalue (AI|GetBlackboard 0))
  (bind _attacktargetkeyname (Variables|Default|GetAttackTargetKeyName))
  (bind _returnvalue_2 (AI|Components|Blackboard|GetValueasObject _returnvalue _attacktargetkeyname))
  (if (Utilities|IsValid _returnvalue_2)
    (bind _isdead (Class|RTSIBPDamageable|IsDead(Message) _returnvalue_2))
    (if _isdead
      _
      (else
        (Class|AIPerceptionComponent|ForgetAll (Variables|Default|GetAIPerception))
        (return))))
  (bind _isdead_2 (Class|RTSIBPDamageable|IsDead(Message) TargetToFollow))
  (if _isdead_2
    (AI|Components|Blackboard|ClearValue (AI|GetBlackboard 0) (Variables|Default|GetAttackTargetKeyName))
    (Class|AIPerceptionComponent|ForgetAll (Variables|Default|GetAIPerception))
    (return)
    (else
      (AI|Components|Blackboard|SetValueasObject (AI|GetBlackboard 0) (Variables|Default|GetAttackTargetKeyName) TargetToFollow)
      (Class|AIPerceptionComponent|ForgetAll (Variables|Default|GetAIPerception))
      (return))))

(fn ClicktoAttack
  (params (ClickToAttackTarget :type Actor%20Object%20Reference))
  (Utilities|IsValid ClickToAttackTarget
    (:Is%20Valid
      (bind _isdead (Class|RTSIBPDamageable|IsDead(Message) ClickToAttackTarget))
      (if _isdead
        (return)
        (else
          (AI|Components|Blackboard|SetValueasObject (AI|GetBlackboard 0) (Variables|Default|GetAttackTargetKeyName) ClickToAttackTarget)
          (return))))
    (:Is%20Not%20Valid
      (return))))

(fn GrabSelectedUnits
  (return 0))