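; AI controller for goblin worker units in the RTS, running RTS_GoblinBT and seeding drop point and main building blackboard keys from tagged actors.
; AI perception routes sensed trees, enemies, resource buildings and meat by tag into blackboard targets.
; Tree, enemy and meat targets persist until invalid or dead, with perception wiped after each check.
; ClickToSetResource overrides the target, switching the unit between wood and food.
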(event OnTargetPerceptionUpdated(AIPerception)
  (params (Actor :type Actor%20Object%20Reference) (Stimulus :type AI%20Stimulus%20Structure))
  (bind _bsuccessfullysensed (Utilities|Struct|BreakAIStimulus Stimulus))
  ;[1 1 1] AI Perception
  (if (Actor|ActorHasTag Actor "Tree")
    (if _bsuccessfullysensed
      (bind _isdead (Class|RTSIBPDamageable|IsDead(Message) Actor))
      (if (not _isdead)
        (CallFunction|FollowNewTree Actor)))
    (elif (Actor|ActorHasTag Actor "EnemyUnit")
      (if _bsuccessfullysensed
        (bind _isdead_2 (Class|RTSIBPDamageable|IsDead(Message) Actor))
        (if (not _isdead_2)
          (CallFunction|RunAwayfromEnemy Actor)))
      (elif (Actor|ActorHasTag Actor "ResourceBuilding")
        (if _bsuccessfullysensed
          (bind _isdead_3 (Class|RTSIBPDamageable|IsDead(Message) Actor))
          (if (not _isdead_3)
            (CallFunction|FollowResourceBuilding Actor)))
        (elif (Actor|ActorHasTag Actor "Meat")
          (if _bsuccessfullysensed
            (bind _isdead_4 (Class|RTSIBPDamageable|IsDead(Message) Actor))
            (if (not _isdead_4)
              (CallFunction|FollowMeat Actor))))))))

(event EventBeginPlay
  ;[1 1 1] Run BT and Initialize the Main Building Location
  (AI|RunBehaviorTree "/Game/OrcLaborContent/Blueprints/Unit_AI/RTS_GoblinBT.RTS_GoblinBT")
  (bind _outactors (Actor|GetAllActorswithTag "DropPoint"))
  (for _array_element _outactors
    _)
  (AI|Components|Blackboard|SetValueasObject (AI|GetBlackboard 0) (Variables|Default|GetResourceBuildingKey) _array_element)
  (bind _outactors_2 (Actor|GetAllActorswithTag "MainBuilding"))
  (for _array_element_2 _outactors_2
    _)
  (AI|Components|Blackboard|SetValueasObject (AI|GetBlackboard 0) (Variables|Default|GetMainBuilding) _array_element_2))

(fn ConstructionScript)

(fn FollowNewTree
  (params (TargetToFollow :type Object%20Object%20Reference))
  (bind _returnvalue (AI|GetBlackboard 0))
  (bind _treetarget (Variables|Default|GetTreeTarget))
  (bind _returnvalue_2 (AI|Components|Blackboard|GetValueasObject _returnvalue _treetarget))
  (if (Utilities|IsValid _returnvalue_2)
    (bind _isdead (Class|RTSIBPDamageable|IsDead(Message) _returnvalue_2))
    (if _isdead
      _
      (else
        (Class|AIPerceptionComponent|ForgetAll (Variables|Default|GetAIPerception))
        (return))))
  (bind _isdead_2 (Class|RTSIBPDamageable|IsDead(Message) TargetToFollow))
  (if _isdead_2
    (AI|Components|Blackboard|ClearValue (AI|GetBlackboard 0) (Variables|Default|GetTreeTarget))
    (Class|AIPerceptionComponent|ForgetAll (Variables|Default|GetAIPerception))
    (return)
    (else
      (AI|Components|Blackboard|SetValueasObject (AI|GetBlackboard 0) (Variables|Default|GetTreeTarget) TargetToFollow)
      (Class|AIPerceptionComponent|ForgetAll (Variables|Default|GetAIPerception))
      (return))))

(fn RunAwayfromEnemy
  (params (TargetToFollow :type Object%20Object%20Reference))
  (bind _returnvalue (AI|GetBlackboard 0))
  (bind _enemytarget (Variables|Default|GetEnemyTarget))
  (bind _returnvalue_2 (AI|Components|Blackboard|GetValueasObject _returnvalue _enemytarget))
  (if (Utilities|IsValid _returnvalue_2)
    (bind _isdead (Class|RTSIBPDamageable|IsDead(Message) _returnvalue_2))
    (if _isdead
      _
      (else
        (Class|AIPerceptionComponent|ForgetAll (Variables|Default|GetAIPerception))
        (return))))
  (bind _isdead_2 (Class|RTSIBPDamageable|IsDead(Message) TargetToFollow))
  (if _isdead_2
    (AI|Components|Blackboard|ClearValue (AI|GetBlackboard 0) (Variables|Default|GetEnemyTarget))
    (Class|AIPerceptionComponent|ForgetAll (Variables|Default|GetAIPerception))
    (return)
    (else
      (AI|Components|Blackboard|SetValueasObject (AI|GetBlackboard 0) (Variables|Default|GetEnemyTarget) TargetToFollow)
      (Class|AIPerceptionComponent|ForgetAll (Variables|Default|GetAIPerception))
      (return))))

(fn FollowResourceBuilding
  (params (TargetToFollow :type Object%20Object%20Reference))
  (AI|Components|Blackboard|SetValueasObject (AI|GetBlackboard 0) (Variables|Default|GetResourceBuildingKey) TargetToFollow)
  (return))

(fn FollowMeat
  (params (TargetToFollow :type Object%20Object%20Reference))
  (bind _returnvalue (AI|GetBlackboard 0))
  (bind _foodtarget (Variables|Default|GetFoodTarget))
  (bind _returnvalue_2 (AI|Components|Blackboard|GetValueasObject _returnvalue _foodtarget))
  (if (Utilities|IsValid _returnvalue_2)
    (bind _isdead (Class|RTSIBPDamageable|IsDead(Message) _returnvalue_2))
    (if _isdead
      _
      (else
        (Class|AIPerceptionComponent|ForgetAll (Variables|Default|GetAIPerception))
        (return))))
  (bind _isdead_2 (Class|RTSIBPDamageable|IsDead(Message) TargetToFollow))
  (if _isdead_2
    (AI|Components|Blackboard|ClearValue (AI|GetBlackboard 0) (Variables|Default|GetFoodTarget))
    (Class|AIPerceptionComponent|ForgetAll (Variables|Default|GetAIPerception))
    (return)
    (else
      (AI|Components|Blackboard|SetValueasObject (AI|GetBlackboard 0) (Variables|Default|GetFoodTarget) TargetToFollow)
      (Class|AIPerceptionComponent|ForgetAll (Variables|Default|GetAIPerception))
      (return))))

(fn ClicktoSetResource
  (params (TargetResource :type Actor%20Object%20Reference))
  (if (Actor|ActorHasTag TargetResource "Tree")
    (AI|Components|Blackboard|ClearValue (AI|GetBlackboard 0) (Variables|Default|GetTreeTarget))
    (AI|Components|Blackboard|SetValueasObject (AI|GetBlackboard 0) (Variables|Default|GetTreeTarget) TargetResource)
    (AI|Components|Blackboard|SetValueasBool (AI|GetBlackboard 0) (Variables|Default|GetTargetIsWood) true)
    (AI|Components|Blackboard|ClearValue (AI|GetBlackboard 0) (Variables|Default|GetTargetIsFood))
    (AI|Components|Blackboard|ClearValue (AI|GetBlackboard 0) (Variables|Default|GetFoodTarget))
    (return)
    (elif (Actor|ActorHasTag TargetResource "Meat")
      (AI|Components|Blackboard|ClearValue (AI|GetBlackboard 0) (Variables|Default|GetFoodTarget))
      (AI|Components|Blackboard|SetValueasObject (AI|GetBlackboard 0) (Variables|Default|GetFoodTarget) TargetResource)
      (AI|Components|Blackboard|SetValueasBool (AI|GetBlackboard 0) (Variables|Default|GetTargetIsFood) true)
      (AI|Components|Blackboard|ClearValue (AI|GetBlackboard 0) (Variables|Default|GetTargetIsWood))
      (AI|Components|Blackboard|ClearValue (AI|GetBlackboard 0) (Variables|Default|GetTreeTarget))
      (return))))

(fn GrabSelectedUnits
  (return 0))