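; AI controller for a melee RTS unit that senses and targets player units, the main building and other buildings.
; On BeginPlay it runs the RTS_ELFMeleeBT behavior tree and stores a MainBuilding-tagged actor in the blackboard.
; AI Perception sorts living sensed actors by tag into separate attack blackboard keys.
; A unit target is replaced only when invalid or dead, and perception is cleared after each unit evaluation.
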(event OnTargetPerceptionUpdated(AIPerception)
  (params (Actor :type Actor%20Object%20Reference) (Stimulus :type AI%20Stimulus%20Structure))
  (bind _bsuccessfullysensed (Utilities|Struct|BreakAIStimulus Stimulus))
  ;[1 1 1] AI Perception
  (if (Actor|ActorHasTag Actor "PlayerUnit")
    (if _bsuccessfullysensed
      (bind _isdead (Class|RTSIBPDamageable|IsDead(Message) Actor))
      (if (not _isdead)
        (CallFunction|FollowNewPlayerUnit Actor)))
    (elif (Actor|ActorHasTag Actor "MainBuilding")
      (if _bsuccessfullysensed
        (bind _isdead_2 (Class|RTSIBPDamageable|IsDead(Message) Actor))
        (if (not _isdead_2)
          (CallFunction|FollowMainBuilding Actor)))
      (elif (Actor|ActorHasTag Actor "Building")
        (if _bsuccessfullysensed
          (bind _isdead_3 (Class|RTSIBPDamageable|IsDead(Message) Actor))
          (if (not _isdead_3)
            (CallFunction|FollowOtherBuilding Actor)))))))

(event EventBeginPlay
  ;[1 1 1] Run BT and Initialize the Main Building Location
  (AI|RunBehaviorTree "/Game/OrcLaborContent/Blueprints/Unit_AI/RTS_ELFMeleeBT.RTS_ELFMeleeBT")
  (bind _outactors (Actor|GetAllActorswithTag "MainBuilding"))
  (for _array_element _outactors
    _)
  (AI|Components|Blackboard|SetValueasObject (AI|GetBlackboard 0) (Variables|Default|GetMainBuilding) _array_element))

(fn ConstructionScript)

(fn FollowNewPlayerUnit
  (params (TargetToFollow :type Object%20Object%20Reference))
  (bind _returnvalue (AI|GetBlackboard 0))
  (bind _attacktargetkeyname (Variables|Default|GetAttackTargetKeyName))
  (bind _returnvalue_2 (AI|Components|Blackboard|GetValueasObject _returnvalue _attacktargetkeyname))
  (if (Utilities|IsValid _returnvalue_2)
    (bind _isdead (Class|RTSIBPDamageable|IsDead(Message) _returnvalue_2))
    (if _isdead
      _
      (else
        (Class|AIPerceptionComponent|ForgetAll (Variables|Default|GetAIPerception))
        (return))))
  (bind _isdead_2 (Class|RTSIBPDamageable|IsDead(Message) TargetToFollow))
  (if _isdead_2
    (AI|Components|Blackboard|ClearValue (AI|GetBlackboard 0) (Variables|Default|GetAttackTargetKeyName))
    (Class|AIPerceptionComponent|ForgetAll (Variables|Default|GetAIPerception))
    (return)
    (else
      (AI|Components|Blackboard|SetValueasObject (AI|GetBlackboard 0) (Variables|Default|GetAttackTargetKeyName) TargetToFollow)
      (Class|AIPerceptionComponent|ForgetAll (Variables|Default|GetAIPerception))
      (return))))

(fn FollowMainBuilding
  (params (TargetToFollow :type Object%20Object%20Reference))
  (AI|Components|Blackboard|SetValueasObject (AI|GetBlackboard 0) (Variables|Default|GetAttackMainBuildingKeyName) TargetToFollow)
  (return))

(fn FollowOtherBuilding
  (params (TargetToFollow :type Object%20Object%20Reference))
  (AI|Components|Blackboard|SetValueasObject (AI|GetBlackboard 0) (Variables|Default|GetAttackBuildingKeyName) TargetToFollow)
  (return))

(fn GrabSelectedUnits
  (return 0))