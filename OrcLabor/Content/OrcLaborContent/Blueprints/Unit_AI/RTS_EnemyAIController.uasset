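; AI controller for RTS enemy units that picks player units and buildings as attack targets.
; On BeginPlay it runs the RTS_EnemyBT behavior tree and stores the last actor tagged MainBuilding in the blackboard.
; AI perception sorts successfully sensed actors by tag (PlayerUnit, then MainBuilding, then Building) and writes each to its own attack blackboard key.
; Lost sightings leave those keys untouched, and GrabSelectedUnits is an empty stub.
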(event OnTargetPerceptionUpdated(AIPerception)
  (params (Actor :type Actor%20Object%20Reference) (Stimulus :type AI%20Stimulus%20Structure))
  (bind _bsuccessfullysensed (Utilities|Struct|BreakAIStimulus Stimulus))
  (if (Actor|ActorHasTag Actor "PlayerUnit")
    (if _bsuccessfullysensed
      (CallFunction|FollowNewPlayerUnit Actor))
    (elif (Actor|ActorHasTag Actor "MainBuilding")
      (if _bsuccessfullysensed
        (CallFunction|FollowMainBuilding Actor))
      (elif (Actor|ActorHasTag Actor "Building")
        (if _bsuccessfullysensed
          (CallFunction|FollowOtherBuilding Actor))))))

(event EventBeginPlay
  ;[1 1 1] Run BT and Initialize the Main Building Location
  (AI|RunBehaviorTree "/Game/OrcLaborContent/Blueprints/Unit_AI/RTS_EnemyBT.RTS_EnemyBT")
  (bind _outactors (Actor|GetAllActorswithTag "MainBuilding"))
  (for _array_element _outactors
    _)
  (AI|Components|Blackboard|SetValueasObject (AI|GetBlackboard 0) (Variables|Default|GetMainBuilding) _array_element))

(fn ConstructionScript)

(fn FollowNewPlayerUnit
  (params (TargetToFollow :type Object%20Object%20Reference))
  (AI|Components|Blackboard|SetValueasObject (AI|GetBlackboard 0) (Variables|Default|GetAttackTargetKeyName) TargetToFollow)
  (return))

(fn FollowMainBuilding
  (params (TargetToFollow :type Object%20Object%20Reference))
  (AI|Components|Blackboard|SetValueasObject (AI|GetBlackboard 0) (Variables|Default|GetAttackMainBuildingKeyName) TargetToFollow)
  (return))

(fn FollowOtherBuilding
  (params (TargetToFollow :type Object%20Object%20Reference))
  (AI|Components|Blackboard|SetValueasObject (AI|GetBlackboard 0) (Variables|Default|GetAttackBuildingKeyName) TargetToFollow)
  (return))

(fn GrabSelectedUnits
  (return 0))