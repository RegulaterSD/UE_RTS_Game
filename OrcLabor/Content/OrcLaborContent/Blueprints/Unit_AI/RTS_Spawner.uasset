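; RTS enemy wave spawner that places alternating Elf Fighters and Rangers at random navigable points around itself.
; Regular waves trigger when wave points pass a rising threshold and none is running; big waves skip both checks, and both scale size with points.
; Each wave updates the resource manager's counter, shows an alert, and swaps day music for battle music until polling finds no EnemyUnit actors.
; The timed spawn loop is disabled.
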(event Custom|Spawn
  ;[1 1 1] Spawn Sequence
  (bind _randomlocation (Class|NavigationSystemV1|GetRandomLocationinNavigableRadius (Transformation|GetActorLocation) (Math|Conversions|ToFloat(Integer) (Variables|Default|GetSpawnRadius)) 0 0))
  (Utilities|FlowControl|FlipFlop
    (:A
      (Game|SpawnActorfromClass "/Game/OrcLaborContent/Blueprints/Units/Enemy_ElfFighter.Enemy_ElfFighter_C" (Math|Transform|MakeTransform (Math|Vector|MakeVector (.X (Math|Vector|BreakVector _randomlocation)) (.Y (Math|Vector|BreakVector _randomlocation)) (+ (.Z (Math|Vector|BreakVector _randomlocation)) 8e+01)) "0, 0, 0" "1.000000,1.000000,1.000000") "Undefined" "MultiplyWithRoot" 0 5e+01 1e+02 0))
    (:B
      (Game|SpawnActorfromClass "/Game/OrcLaborContent/Blueprints/Units/Enemy_ElfRanger.Enemy_ElfRanger_C" (Math|Transform|MakeTransform (Math|Vector|MakeVector (.X (Math|Vector|BreakVector _randomlocation)) (.Y (Math|Vector|BreakVector _randomlocation)) (+ (.Z (Math|Vector|BreakVector _randomlocation)) 8e+01)) "0, 0, 0" "1.000000,1.000000,1.000000") "Undefined" "MultiplyWithRoot" 0 5e+01 1e+02 0))))

(event Custom|Loop
  ;[0 0 0] Loop Sequence (Disabled)
)

(event Custom|BigWave
  ;[1 1 1] Big Wave
  (Variables|Default|SetWave (+ (Variables|Default|GetWave) 1))
  (Default|UpdateWaveCounter (Variables|Default|GetResource%20Manager))
  (Variables|Default|SetWave%20Point%20Iterator (+ (Variables|Default|GetWave%20Point%20Iterator) 1))
  (Default|ShowWaveAlert (Variables|Default|GetAlertUI))
  (Audio|PlaySound2D "/Game/OrcLaborContent/Assets/Audio/SFX/Voices/Orc_Pack/angry3.angry3" 1.0 1.0 0.0 0 0)
  (for _index (range 1 (Math|Integer|Max(Integer) (* (Variables|/Game/OrcLaborContent/Blueprints/Resources/RTS_Resource_Manager.RTS_Resource_Manager_C|GetPoints (Variables|Default|GetResource%20Manager)) (Variables|Default|GetBig%20Wave%20Point%20Size%20Multiplier)) 1)) ; Spawn Enemies
    (CallFunction|Spawn))
  (Utilities|WaitforWaveClear (Variables|Default|GetBigWaveMusic)))

(event Custom|Wave%20based%20on%20Wave%20Points
  (params (Wave%20Points :type Integer) (Points :type Integer))
  ;[1 1 1] Wave Based on Points
  (if (not (Variables|Default|GetWaveInProgress)) ; Cancel spawn if there's a wave in progress
    (if (>= Wave%20Points (* (Variables|Default|GetWave%20Point%20Iterator) (Variables|Default|GetWave%20Point%20Interval)))
      (Variables|Default|SetWave (+ (Variables|Default|GetWave) 1))
      (Default|UpdateWaveCounter (Variables|Default|GetResource%20Manager))
      (Variables|Default|SetWave%20Point%20Iterator (+ (Variables|Default|GetWave%20Point%20Iterator) 1))
      (Default|ShowWaveAlert (Variables|Default|GetAlertUI))
      (Audio|PlaySound2D "/Game/OrcLaborContent/Assets/Audio/SFX/Voices/Orc_Pack/angry2.angry2" 1.0 1.0 0.0 0 0)
      (for _index (range 1 (Math|Integer|Max(Integer) (* Points (Variables|Default|GetWave%20Point%20Size%20Multiplier)) 1)) ; Spawn Enemies
        (CallFunction|Spawn))
      (Utilities|WaitforWaveClear (Variables|Default|GetBasicWaveMusic)))))

(event EventBeginPlay
  ;[1 1 1] Initialize Music
  (bind _returnvalue (Audio|SpawnSound2D "/Game/OrcLaborContent/Assets/Audio/SFX/Loops/Forest_Day/Forest_Day.Forest_Day" 1.0 1.0 0.0 0))
  (Variables|Default|SetDayMusic _returnvalue)
  ;[1 1 1] Initialize Resource Manager
  (bind _returnvalue_2 (Actor|GetActorOfClass "/Game/OrcLaborContent/Blueprints/Resources/RTS_Resource_Manager.RTS_Resource_Manager_C"))
  (Variables|Default|SetResource%20Manager _returnvalue_2)
  ;[1 1 1] Initialize Alert UI
  (bind _returnvalue_3 (UserInterface|CreateWidget "/Game/OrcLaborContent/Blueprints/UI/WB_AlertUI.WB_AlertUI_C"))
  (bind _output_get (Variables|Default|SetAlertUI _returnvalue_3))
  (UserInterface|Viewport|AddtoViewport _output_get 0))

(fn ConstructionScript)

(fn GrabSelectedUnits
  (return 0))