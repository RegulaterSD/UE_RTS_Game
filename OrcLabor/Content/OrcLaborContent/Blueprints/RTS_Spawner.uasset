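; RTS_Spawner is an RTS spawner actor that spawns waves of enemies around itself, starting at BeginPlay.
; A self-calling Loop event spawns the current batch, waits a set delay, then repeats indefinitely.
; Each spawn lands at a random navigable point within the spawn radius, raised slightly above it.
; An iteration counter grows the batch by one enemy after a configurable number of waves.
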(event Custom|Spawn
  ;[1 1 1] Spawn Sequence
  (bind _randomlocation (Class|NavigationSystemV1|GetRandomLocationinNavigableRadius (Transformation|GetActorLocation) (Math|Conversions|ToFloat(Integer) (Variables|Default|GetSpawnRadius)) 0 0))
  (Game|SpawnActorfromClass "/Game/OrcLaborContent/Blueprints/Units/Enemy_ElfRanger.Enemy_ElfRanger_C" (Math|Transform|MakeTransform (Math|Vector|MakeVector (.X (Math|Vector|BreakVector _randomlocation)) (.Y (Math|Vector|BreakVector _randomlocation)) (+ (.Z (Math|Vector|BreakVector _randomlocation)) 8e+01)) "0, 0, 0" "1.000000,1.000000,1.000000") "Undefined" "MultiplyWithRoot" 0 5e+01 1e+02 0))

(event Custom|Loop
  ;[1 1 1] Loop Sequence
  (for _index (range 1 (Variables|Default|GetInitSpawnAmount))
    (CallFunction|Spawn))
  (Utilities|FlowControl|Delay (Math|Conversions|ToFloat(Integer) (Variables|Default|GetSpawnWaitTime)))
  (if (>= (Variables|Default|GetLoopIterator) (- (Variables|Default|GetSpawnIncreaseIteration) 1))
    (Variables|Default|SetLoopIterator 0)
    (Variables|Default|SetInitSpawnAmount (+ (Variables|Default|GetInitSpawnAmount) 1)) ; After "x" amount of loops, increase the number of enemies that spawn by 1
    (else
      (Variables|Default|SetLoopIterator (+ (Variables|Default|GetLoopIterator) 1))))
  (CallFunction|Loop))

(event EventBeginPlay
  (CallFunction|Loop))

(fn ConstructionScript)