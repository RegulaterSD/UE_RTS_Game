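; Production building for an RTS that offers Orc Warrior production through the action box and can take damage.
; On BeginPlay it creates the Orc Warrior production button widget, links it to itself and registers it in ActionBoxButtons before calling the parent.
; Damage, healing, health and death queries forward to the RTS damage system component, whose death and damage-response events bind at construction.
; Taking damage also updates the building bar's current health.
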(event EventBeginPlay
  ;[1 1 1] Unit Production Types (Action Box)
  (Utilities|FlowControl|Sequence
    (:then_0
      (bind _returnvalue (UserInterface|CreateWidget "/Game/OrcLaborContent/Blueprints/UI/WB_Produce_OrcWarrior.WB_Produce_OrcWarrior_C"))
      (Utilities|Array|AddUnique (Variables|Default|GetActionBoxButtons) _returnvalue)
      (Variables|/Game/OrcLaborContent/Blueprints/UI/WB_Produce_OrcWarrior.WB_Produce_OrcWarrior_C|SetBuildingRef _returnvalue self))
    (:then_2
      (|CallParentFunction))))

(event Collision|EventActorBeginOverlap
  (params (OtherActor :type Actor%20Object%20Reference))
  (|CallParentFunction OtherActor) ; This node is disabled and will not be called.\nDrag off pins to build functionality.
)

(event EventTick
  (params (DeltaSeconds :type Float%20%28single-precision%29))
  (|CallParentFunction DeltaSeconds) ; This node is disabled and will not be called.\nDrag off pins to build functionality.
)

(fn ConstructionScript
  (bind _rts_bpc_damagesystem (Variables|Default|GetRTS_BPC_DamageSystem))
  (EventDispatchers|BindEventtoOnDeath _rts_bpc_damagesystem (EventDispatchers|CreateEvent :!event Death))
  (EventDispatchers|BindEventtoOnDamageResponse _rts_bpc_damagesystem (EventDispatchers|CreateEvent :!event DamageResponse)))

(fn IsDead
  (return (Variables|/Game/OrcLaborContent/Blueprints/DamageSystem/RTS_BPC_DamageSystem.RTS_BPC_DamageSystem_C|GetIsDead (Variables|Default|GetRTS_BPC_DamageSystem))))

(fn TakeDamage
  (params (DamageInfo :type RTS%20S%20Damage%20Info%20Structure))
  (bind _wasdamaged (Default|TakeDamage (Variables|Default|GetRTS_BPC_DamageSystem) DamageInfo))
  (bind _health (CallFunction|GetCurrentHealth))
  (Variables|/Game/OrcLaborContent/Blueprints/UI/WB_BuildingStatusBar.WB_BuildingStatusBar_C|SetCurrentHealth (Variables|Default|GetBuildingBarReference) _health)
  (return _wasdamaged))

(fn Heal
  (params (AmountToHeal :type Float%20%28double-precision%29))
  (bind _newhealth (Default|Heal (Variables|Default|GetRTS_BPC_DamageSystem) AmountToHeal))
  (return _newhealth))

(fn GetMaxHealth
  (return (Variables|/Game/OrcLaborContent/Blueprints/DamageSystem/RTS_BPC_DamageSystem.RTS_BPC_DamageSystem_C|GetMaxHealth (Variables|Default|GetRTS_BPC_DamageSystem))))

(fn GetCurrentHealth
  (return (Variables|/Game/OrcLaborContent/Blueprints/DamageSystem/RTS_BPC_DamageSystem.RTS_BPC_DamageSystem_C|GetHealth (Variables|Default|GetRTS_BPC_DamageSystem))))