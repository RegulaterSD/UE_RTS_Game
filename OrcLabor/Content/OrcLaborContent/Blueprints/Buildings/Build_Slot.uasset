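; Build_Slot is a clickable land plot where the player builds a structure in exchange for wood.
; BeginPlay enables click and mouse-over events on the player controller.
; Clicking an unbuilt slot destroys its highlight decal, asks the RTS_Resource_Manager to spend the cost, and on success spawns the BuildingMesh class at the slot's transform and marks it built.
; The decal is removed even when payment fails, and feedback is debug prints only.
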(event OnClicked(land)
  (params (TouchedComponent :type Primitive%20Component%20Object%20Reference) (ButtonPressed :type Key%20Structure))
  (bind _returnvalue (Transformation|GetActorTransform))
  (bind (_location _rotation _scale) (Math|Transform|BreakTransform _returnvalue))
  (bind (_x _y _z) (Math|Vector|BreakVector _location))
  ;[1 1 1] On Click
  (Development|PrintString "Clicked on land")
  (if (Variables|Default|GetBuilt)
    (Development|PrintString "Structure already built")
    (else
      (Components|DestroyComponent (Variables|Default|GetHighlightDecal))
      (bind _returnvalue_2 (Actor|GetActorOfClass "/Game/OrcLaborContent/Blueprints/Resources/RTS_Resource_Manager.RTS_Resource_Manager_C"))
      (bind _can_build (Default|SpendWood _returnvalue_2 (Variables|Default|GetCost)))
      (if _can_build
        (Game|SpawnActorfromClass (Variables|Default|GetBuildingMesh) (Math|Transform|MakeTransform (Math|Vector|MakeVector _x _y (+ _z 0.0)) _rotation _scale) "Undefined" "MultiplyWithRoot" 0 0)
        (Variables|Default|SetBuilt true)
        (Development|PrintString "Structure Built")
        (else
          (Development|PrintString "cant build"))))))

(event OnBeginCursorOver(land)
  (params (TouchedComponent :type Primitive%20Component%20Object%20Reference))
  ;[1 1 1] Over Land
  (Development|PrintString "Mouse over land"))

(event EventBeginPlay
  (bind _returnvalue (Game|GetPlayerController 0))
  ;[1 1 1] Set up events
  (Variables|/Script/Engine.PlayerController|SetbEnableClickEvents _returnvalue true)
  (Variables|/Script/Engine.PlayerController|SetbEnableMouseOverEvents _returnvalue true))

(fn ConstructionScript)