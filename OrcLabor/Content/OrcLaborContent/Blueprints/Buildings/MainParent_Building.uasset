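; Parent Blueprint for RTS buildings, providing selection, health and damage handling, and unit production.
; Selection toggles a decal and a production widget populated with action buttons.
; Health and damage calls forward to RTSBPCDamageSystem, with a status bar showing health and particle effects on damage responses.
; A looping timer advances the production queue one unit at a time using each class's default ProductionTime, spawning finished units at UnitSpawnPoint.
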(event Custom|AddUnitToQuene
  (params (Unit :type Player%20Unit%20Class%20Reference))
  ;[1 1 1] Unit Prodution
  ;;[0.2232 0.2232 0.2232] Add Unit to Quene
  (Utilities|Array|Add (Variables|Default|GetUnitProducionQueue) Unit))

(event Custom|OnDeath
  ;[1 1 1] OnDeath
)

(event Custom|ProcessProductionQueue
  ;[1 1 1] Unit Prodution
  ;;[0.2232 0.2232 0.2232] Production Queue
  (if (Variables|Default|GetIsProducing)
    ;;[0.2232 0.2232 0.2232] True Side
    (bind _output_get (Variables|Default|SetProductionTimeSpent (+ (Variables|Default|GetProductionTimeSpent) (Variables|Default|GetProductionTimerGranularity))))
    (bind _output_get_2 (Variables|Default|SetProductionProgress (/ _output_get (Variables|Default|GetProductionTimeNeeded))))
    (if (>= _output_get_2 1.0)
      ;;[0.2232 0.2232 0.2232] Unit Spawn
      (Game|SpawnActorfromClass (Variables|Default|GetUnitBeingProduced) (Math|Transform|MakeTransform (Transformation|GetWorldLocation (Variables|Default|GetUnitSpawnPoint)) "0, 0, 0" "1.000000,1.000000,1.000000") "AdjustIfPossibleButAlwaysSpawn" "MultiplyWithRoot" 0 5e+01 1e+02 0)
      (Variables|Default|SetProductionProgress 0.0)
      (Variables|Default|SetProductionTimeSpent 0.0)
      (Variables|Default|SetUnitBeingProduced 0)
      (Variables|Default|SetIsProducing false))
    (else
      ;;[0.2232 0.2232 0.2232] False Side
      (if (> (Utilities|Array|Length (Variables|Default|GetUnitProducionQueue)) 0)
        (bind _output_get_3 (Variables|Default|SetUnitBeingProduced (Utilities|Array|Get(acopy) (Variables|Default|GetUnitProducionQueue))))
        (Variables|Default|SetProductionTimeNeeded (.ProductionTime (Utilities|GetClassDefaults _output_get_3)))
        (Utilities|Array|RemoveIndex (Variables|Default|GetUnitProducionQueue))
        (Variables|Default|SetIsProducing true)))))

(event Custom|Death
  ;[1 1 1] Death Function
  (Effects|SpawnEmitteratLocation "/Game/MarketplaceContent/Realistic_Starter_VFX_Pack_Vol2/Particles/Explosion/P_Explosion_Big_A.P_Explosion_Big_A" (Transformation|GetActorLocation) "0, 0, 0" "7.500000,7.500000,7.500000")
  (Actor|DestroyActor))

(event Custom|DamageResponse
  (params (DamageResponse :type RTS_ENUM_DamageResponse%20Enum :default "NewEnumerator0"))
  ;[1 1 1] Damage Type
  (Effects|SpawnEmitterAttached "/Game/MarketplaceContent/Realistic_Starter_VFX_Pack_Vol2/Particles/Hit/P_Brick.P_Brick" (Variables|Default|GetBuildingMesh) "None" "0.000000,0.000000,10.000000" "0, 0, 0" "8.500000,8.500000,8.500000"))

(event Game|Damage|EventAnyDamage
  (params (Damage :type Float%20%28single-precision%29) (DamageType :type Damage%20Type%20Object%20Reference) (InstigatedBy :type Controller%20Object%20Reference) (DamageCauser :type Actor%20Object%20Reference))
  (bind _buildingbarreference (Variables|Default|GetBuildingBarReference))
  ;[1 1 1] Basic Damage Reference
  (Variables|/Game/OrcLaborContent/Blueprints/UI/WB_BuildingStatusBar.WB_BuildingStatusBar_C|SetCurrentHealth _buildingbarreference (stale EventBeginPlay _health))
  (Variables|/Game/OrcLaborContent/Blueprints/UI/WB_BuildingStatusBar.WB_BuildingStatusBar_C|SetMaxHealth _buildingbarreference (stale EventBeginPlay _maxhealth)))

(event EventSelectThis
  ;[1 1 1] Building Selection
  (Rendering|SetVisibility (Variables|Default|GetSelectionDecal) true false)
  (UserInterface|Viewport|AddtoViewport (Variables|Default|GetBuildingSelectedWidget) 0))

(event EventDeselectThis
  ;[1 1 1] Building Selection
  (Rendering|SetVisibility (Variables|Default|GetSelectionDecal) false false)
  (Widget|RemovefromParent (Variables|Default|GetBuildingSelectedWidget)))

(event EventBeginPlay
  ;[1 1 1] Event BeginPlay
  (Utilities|FlowControl|Sequence
    (:then_0
      ;[1 1 1] Creat Building Select Widget
      (bind _returnvalue (UserInterface|CreateWidget "/Game/OrcLaborContent/Blueprints/UI/WB_BuildingWidget_Production.WB_BuildingWidget_Production_C"))
      (Variables|Default|SetBuildingSelectedWidget _returnvalue)
      (Variables|/Game/OrcLaborContent/Blueprints/UI/WB_BuildingWidget_Production.WB_BuildingWidget_Production_C|SetBuildingRefrence _returnvalue self)
      (for _array_element (Variables|Default|GetActionBoxButtons)
        (Class|WrapBox|AddChildtoWrapBox (Variables|/Game/OrcLaborContent/Blueprints/UI/WB_BuildingWidget_Production.WB_BuildingWidget_Production_C|GetActionBox (Variables|Default|GetBuildingSelectedWidget)) _array_element)))
    (:then_1
      ;[1 1 1] Status Bar Event
      (bind _aswb_building_status_bar (Utilities|Casting|CastToWB_BuildingStatusBar (UserInterface|GetUserWidgetObject (Variables|Default|GetWidget))))
      (bind _output_get (Variables|Default|SetBuildingBarReference _aswb_building_status_bar))
      ;;[1 1 1] Inital Health Bar
      (bind _health (CallFunction|GetCurrentHealth))
      (Variables|/Game/OrcLaborContent/Blueprints/UI/WB_BuildingStatusBar.WB_BuildingStatusBar_C|SetCurrentHealth _output_get _health)
      (bind _maxhealth (CallFunction|GetMaxHealth))
      (Variables|/Game/OrcLaborContent/Blueprints/UI/WB_BuildingStatusBar.WB_BuildingStatusBar_C|SetMaxHealth _output_get _maxhealth))
    (:then_2
      ;[1 1 1] Unit Prodution
      ;;[0.2232 0.2232 0.2232] Production Queue
      (Utilities|Time|SetTimerbyEvent (delegate Custom|ProcessProductionQueue) (Variables|Default|GetProductionTimerGranularity) true))))

(fn ConstructionScript
  (bind _rts_bpc_damagesystem (Variables|Default|GetRTS_BPC_DamageSystem))
  (EventDispatchers|BindEventtoOnDeath _rts_bpc_damagesystem (EventDispatchers|CreateEvent :!event Custom|Death))
  (EventDispatchers|BindEventtoOnDamageResponse _rts_bpc_damagesystem (EventDispatchers|CreateEvent :!event Custom|DamageResponse)))

(fn GetCurrentHealth
  (return (Variables|/Game/OrcLaborContent/Blueprints/DamageSystem/RTS_BPC_DamageSystem.RTS_BPC_DamageSystem_C|GetHealth (Variables|Default|GetRTS_BPC_DamageSystem))))

(fn GetMaxHealth
  (return (Variables|/Game/OrcLaborContent/Blueprints/DamageSystem/RTS_BPC_DamageSystem.RTS_BPC_DamageSystem_C|GetMaxHealth (Variables|Default|GetRTS_BPC_DamageSystem))))

(fn GrabSelectedUnits
  (return 0))

(fn Heal
  (params (AmountToHeal :type Float%20%28double-precision%29))
  (bind _newhealth (Default|Heal (Variables|Default|GetRTS_BPC_DamageSystem) 0.0))
  (return _newhealth))

(fn IsDead
  (return (Variables|/Game/OrcLaborContent/Blueprints/DamageSystem/RTS_BPC_DamageSystem.RTS_BPC_DamageSystem_C|GetIsDead (Variables|Default|GetRTS_BPC_DamageSystem))))

(fn TakeDamage
  (params (DamageInfo :type RTS%20S%20Damage%20Info%20Structure))
  (bind _wasdamaged (Default|TakeDamage (Variables|Default|GetRTS_BPC_DamageSystem) DamageInfo))
  (return _wasdamaged))