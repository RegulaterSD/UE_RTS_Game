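; Parent Blueprint for a harvestable tree that grants wood to the player when clicked.
; BeginPlay enables click and mouse-over events on the first player controller.
; The first click destroys the tree mesh, toggles the stump's visibility, adds WoodGiven to the RTS_Resource_Manager found by class, and sets WoodHarvested to block repeat harvests.
; GrabSelectedUnits is an empty stub, so harvesting involves no units.
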(event EventBeginPlay
  (bind _returnvalue (Game|GetPlayerController 0))
  ;[1 1 1] Set up events
  (Variables|/Script/Engine.PlayerController|SetbEnableClickEvents _returnvalue true)
  (Variables|/Script/Engine.PlayerController|SetbEnableMouseOverEvents _returnvalue true))

(event MouseInput|EventActorOnClicked
  (params (ButtonPressed :type Key%20Structure :default "None"))
  ;[1 1 1] On Click
  (if (not (Variables|Default|GetWoodHarvested))
    (Components|DestroyComponent (Variables|Default|GetStaticMesh_Tree))
    (Rendering|ToggleVisibility (Variables|Default|GetStaticMesh_Stump) false)
    (bind _returnvalue (Actor|GetActorOfClass "/Game/OrcLaborContent/Blueprints/Resources/RTS_Resource_Manager.RTS_Resource_Manager_C"))
    (Default|AddWood _returnvalue (Variables|Default|GetWoodGiven))
    (Variables|Default|SetWoodHarvested true)))

(fn ConstructionScript)

(fn GrabSelectedUnits
  (return 0))