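; RTS resource manager that tracks the player's wood, meat and gold and mirrors them in a WB_ResourceUI widget created at BeginPlay.
; Add functions raise a resource and feed weighted points and wave points, which are pushed to every RTS_Spawner to drive waves.
; Spend functions deduct and return true only when affordable, though SpendGold checks and deducts Meat instead of Gold.
; GrabSelectedUnits is an empty stub.
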(event EventBeginPlay
  (bind _returnvalue (UserInterface|CreateWidget "/Game/OrcLaborContent/Blueprints/UI/WB_ResourceUI.WB_ResourceUI_C"))
  (bind _output_get (Variables|Default|SetResourceUI _returnvalue))
  (UserInterface|Viewport|AddtoViewport _output_get 0))

(fn ConstructionScript)

(fn AddWood
  (params (Wood%20Gathered :type Integer))
  (bind _output_get (Variables|Default|SetWood (+ Wood%20Gathered (Variables|Default|GetWood))))
  (Default|UpdateWOOD (Variables|Default|GetResourceUI) _output_get)
  (CallFunction|UpdatePoints Wood%20Gathered (Variables|Default|GetPoint%20Wood%20Multiplier) (Variables|Default|GetWave%20Wood%20Multiplier)))

(fn SpendWood
  (params (Cost :type Integer))
  (if (< (- (Variables|Default|GetWood) Cost) 0)
    (return false)
    (else
      (bind _output_get (Variables|Default|SetWood (- (Variables|Default|GetWood) Cost)))
      (Default|UpdateWOOD (Variables|Default|GetResourceUI) _output_get)
      (return true))))

(fn AddMeat
  (params (Meat%20Gathered :type Integer))
  (bind _output_get (Variables|Default|SetMeat (+ Meat%20Gathered (Variables|Default|GetMeat))))
  (Default|UpdateMEAT (Variables|Default|GetResourceUI) _output_get)
  (CallFunction|UpdatePoints Meat%20Gathered (Variables|Default|GetPoint%20Meat%20Multiplier) (Variables|Default|GetWave%20Meat%20Multiplier)))

(fn SpendMeat
  (params (Cost :type Integer))
  (if (< (- (Variables|Default|GetMeat) Cost) 0)
    (return false)
    (else
      (bind _output_get (Variables|Default|SetMeat (- (Variables|Default|GetMeat) Cost)))
      (Default|UpdateMEAT (Variables|Default|GetResourceUI) _output_get)
      (return true))))

(fn AddGold
  (params (Gold%20Earned :type Integer))
  (bind _output_get (Variables|Default|SetGold (+ Gold%20Earned (Variables|Default|GetGold))))
  (Default|UpdateGOLD (Variables|Default|GetResourceUI) _output_get)
  (CallFunction|UpdatePoints Gold%20Earned (Variables|Default|GetPoint%20Gold%20Multiplier) (Variables|Default|GetWave%20Gold%20Multiplier)))

(fn SpendGold
  (params (Cost :type Integer))
  (if (< (- (Variables|Default|GetMeat) Cost) 0)
    (return false)
    (else
      (bind _output_get (Variables|Default|SetMeat (- (Variables|Default|GetMeat) Cost)))
      (Default|UpdateGOLD (Variables|Default|GetResourceUI) _output_get)
      (return true))))

(fn UpdatePoints
  (params (Amount :type Integer) (Point%20Multiplier :type Integer) (Wave%20Point%20Multiplier :type Integer))
  (bind _output_get (Variables|Default|SetPoints (+ (* Amount Point%20Multiplier) (Variables|Default|GetPoints))))
  (Default|UpdatePOINTS (Variables|Default|GetResourceUI) _output_get)
  (Variables|Default|SetWavePoints (+ (* Amount Wave%20Point%20Multiplier) (Variables|Default|GetWavePoints)))
  (bind _outactors (Actor|GetAllActorsOfClass "/Game/OrcLaborContent/Blueprints/Unit_AI/RTS_Spawner.RTS_Spawner_C"))
  (for _array_element _outactors
    (Default|WaveBasedonWavePoints _array_element (Variables|Default|GetWavePoints) (Variables|Default|GetPoints))))

(fn GrabSelectedUnits
  (return 0))