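; Meat drop resource actor for an RTS, damageable through an RTS damage system component.
; Damage interface functions forward health and damage calls to the component, though Heal is stubbed, and the construction script binds its death and damage-response delegates.
; Death spawns a blood splat and destroys the actor; DamageResponse is empty.
; BeginPlay enables mouse click and hover events, but the click-to-collect logic that added meat to the resource manager is disconnected.
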(event Custom|OnDeath
  ;[1 1 1] OnDeath
)

(event Custom|Death
  ;[1 1 1] Death Function
  (Effects|SpawnEmitteratLocation "/Game/MarketplaceContent/Realistic_Starter_VFX_Pack_Vol2/Particles/Blood/P_Blood_Splat_Cone.P_Blood_Splat_Cone" (Transformation|GetActorLocation) "0, 0, 0" "2.000000,2.000000,2.000000")
  (Actor|DestroyActor))

(event Custom|DamageResponse
  (params (DamageResponse :type RTS_ENUM_DamageResponse%20Enum :default "NewEnumerator0"))
  ;[1 1 1] Damage Type
)

(event EventBeginPlay
  (bind _returnvalue (Game|GetPlayerController 0))
  ;[1 1 1] Set up events
  (Variables|/Script/Engine.PlayerController|SetbEnableClickEvents _returnvalue true)
  (Variables|/Script/Engine.PlayerController|SetbEnableMouseOverEvents _returnvalue true))

(fn ConstructionScript
  (bind _rts_bpc_damagesystem (Variables|Default|GetRTS_BPC_DamageSystem))
  (EventDispatchers|BindEventtoOnDeath _rts_bpc_damagesystem (EventDispatchers|CreateEvent :!event Custom|Death))
  (EventDispatchers|BindEventtoOnDamageResponse _rts_bpc_damagesystem (EventDispatchers|CreateEvent :!event Custom|DamageResponse)))

(fn GetCurrentHealth
  (return (Variables|/Game/OrcLaborContent/Blueprints/DamageSystem/RTS_BPC_DamageSystem.RTS_BPC_DamageSystem_C|GetHealth (Variables|Default|GetRTS_BPC_DamageSystem))))

(fn GetMaxHealth
  (return (Variables|/Game/OrcLaborContent/Blueprints/DamageSystem/RTS_BPC_DamageSystem.RTS_BPC_DamageSystem_C|GetMaxHealth (Variables|Default|GetRTS_BPC_DamageSystem))))

(fn Heal
  (params (AmountToHeal :type Float%20%28double-precision%29))
  (return 0.0))

(fn IsDead
  (return (Variables|/Game/OrcLaborContent/Blueprints/DamageSystem/RTS_BPC_DamageSystem.RTS_BPC_DamageSystem_C|GetIsDead (Variables|Default|GetRTS_BPC_DamageSystem))))

(fn TakeDamage
  (params (DamageInfo :type RTS%20S%20Damage%20Info%20Structure))
  (bind _wasdamaged (Default|TakeDamage (Variables|Default|GetRTS_BPC_DamageSystem) DamageInfo))
  (return _wasdamaged))