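; Base Blueprint for game units, providing a health status bar and an attack animation.
; On begin play it caches the UnitStatusBar from its widget component, then copies current and max health into it there and on any damage, without changing health itself.
; Attack plays a montage and calls OnAttackFinished whether it completes or is interrupted.
; MoveTo and GrabSelectedUnits are empty here.
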(event Custom|Attack
  ;[1 1 1] Attack Animation
  (Animation|Montage|PlayMontage (Variables|Character|GetMesh) (Variables|Default|GetAttackMontage)
    (:OnCompleted
      _)
    (:OnInterrupted
      _))
  (Default|CallOnAttackFinished))

(event EventBeginPlay
  ;[1 1 1] Status Bar Event
  (bind _asunit_status_bar (Utilities|Casting|CastToUnitStatusBar (UserInterface|GetUserWidgetObject (Variables|Default|GetWidget))))
  (bind _output_get (Variables|Default|SetUnitBarReference _asunit_status_bar))
  ;;[1 1 1] Inital Health Bar
  (Variables|/Game/OrcLaborContent/Blueprints/UI/UnitStatusBar.UnitStatusBar_C|SetCurrentHealth _output_get (Variables|Default|GetCurrentHealth))
  (Variables|/Game/OrcLaborContent/Blueprints/UI/UnitStatusBar.UnitStatusBar_C|SetMaxHealth _output_get (Variables|Default|GetMaxHealth)))

(event Game|Damage|EventAnyDamage
  (params (Damage :type Float%20%28single-precision%29) (DamageType :type Damage%20Type%20Object%20Reference) (InstigatedBy :type Controller%20Object%20Reference) (DamageCauser :type Actor%20Object%20Reference))
  (bind _unitbarreference (Variables|Default|GetUnitBarReference))
  ;[1 1 1] Basic Damage Reference
  (Variables|/Game/OrcLaborContent/Blueprints/UI/UnitStatusBar.UnitStatusBar_C|SetCurrentHealth _unitbarreference (Variables|Default|GetCurrentHealth))
  (Variables|/Game/OrcLaborContent/Blueprints/UI/UnitStatusBar.UnitStatusBar_C|SetMaxHealth _unitbarreference (Variables|Default|GetMaxHealth)))

(fn ConstructionScript)

(fn Moveto
  (params (ToPosition :type Vector)))

(fn GrabSelectedUnits
  (return 0))