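; Enemy archer unit for an RTS-style game, exposing health, heal, damage and attack functions backed by the RTSBPCDamageSystem component.
; Attack toggles the shooting animation, waits a fixed delay, then sphere-traces forward, ignoring EnemyUnit-tagged actors, to damage the hit actor.
; TakeDamage updates the unit bar and signals attack finished.
; Construction binds damage and death events; Death ragdolls the mesh and destroys the actor after a delay.
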(event Custom|Attack
  (bind _returnvalue (Transformation|GetActorLocation))
  ;[1 1 1] Attack Function
  (Audio|SpawnSoundAttached "/Game/OrcLaborContent/Assets/Audio/SFX/Non_Loops/Attacks/Bow_Attacks_Hits_and_Blocks/Bow_Attack_1.Bow_Attack_1" (Variables|Character|GetMesh) "None" "0, 0, 0" "0, 0, 0" "KeepRelativeOffset" false 1.0 1.0 0.0 0 0)
  (bind _isdead (CallFunction|IsDead))
  (if _isdead
    (Default|CallOnAttackFinished)
    (else
      (bind _aself_archer_anim_bp (Utilities|Casting|CastToElf_Archer_Anim_BP (Components|SkeletalMesh|GetAnimInstance (Variables|Character|GetMesh))))
      (Variables|/Game/OrcLaborContent/Assets/Characters/Elf_Ranger/Animations/Elf_Archer_Anim_BP.Elf_Archer_Anim_BP_C|SetisShooting _aself_archer_anim_bp true)
      ;[1 1 1] Geto Fix
      (Utilities|FlowControl|Delay 4.5)
      (Variables|/Game/OrcLaborContent/Assets/Characters/Elf_Ranger/Animations/Elf_Archer_Anim_BP.Elf_Archer_Anim_BP_C|SetisShooting _aself_archer_anim_bp false)
      (bind _outactors (Actor|GetAllActorswithTag "EnemyUnit"))
      (bind (_outhit _returnvalue_2) (Collision|SphereTraceForObjects _returnvalue (+ _returnvalue (* (Transformation|GetActorForwardVector) (Variables|Default|GetAttack%20Distance%20multiplier))) (Variables|Default|GetSphere%20Radius%20for%20Attacking) (Utilities|Array|MakeArray "ObjectTypeQuery3" "ObjectTypeQuery2" "ObjectTypeQuery4" "ObjectTypeQuery5" "ObjectTypeQuery6") false _outactors "None" true "(R=1.000000,G=0.000000,B=0.000000,A=1.000000)" "(R=0.000000,G=1.000000,B=0.000000,A=1.000000)" 1.0))
      (if _returnvalue_2
        (bind _isdead_2 (CallFunction|IsDead))
        (if _isdead_2
          (Default|CallOnAttackFinished)
          (else
            (bind _wasdamaged (Class|RTSIBPDamageable|TakeDamage(Message) (.HitActor (Collision|BreakHitResult _outhit)) (Utilities|Struct|MakeRTS_S_DamageInfo (Variables|Default|GetDamageAmount) (Variables|Default|GetDamage%20Type) "NewEnumerator1")))
            (if _wasdamaged
              (Default|CallOnAttackFinished))))))))

(event Custom|OnDeath
  ;[1 1 1] OnDeath
)

(event Custom|Death
  (bind _mesh (Variables|Character|GetMesh))
  ;[1 1 1] Death Function
  (Development|PrintString "ENemy Unit DEAD")
  (Physics|SetSimulatePhysics _mesh true)
  (Collision|SetCollisionEnabled _mesh "QueryAndPhysics")
  (Utilities|FlowControl|Delay (Variables|Default|GetDeathDelay))
  (Actor|DestroyActor))

(event Custom|DamageResponse
  (params (DamageResponse :type RTS_ENUM_DamageResponse%20Enum :default "NewEnumerator0"))
  ;[1 1 1] Damage Type
  (Audio|SpawnSoundAttached "/Game/OrcLaborContent/Assets/Audio/SFX/Non_Loops/Attacks/Sword_Attacks_Hits_and_Blocks/Sword_Impact_Hit_3.Sword_Impact_Hit_3" (Variables|Character|GetMesh) "None" "0, 0, 0" "0, 0, 0" "KeepRelativeOffset" false 1.0 1.0 0.0 0 0))

(fn ConstructionScript
  (bind _rts_bpc_damagesystem (Variables|Default|GetRTS_BPC_DamageSystem))
  (EventDispatchers|BindEventtoOnDeath _rts_bpc_damagesystem (EventDispatchers|CreateEvent :!event Custom|Death))
  (EventDispatchers|BindEventtoOnDamageResponse _rts_bpc_damagesystem (EventDispatchers|CreateEvent :!event Custom|DamageResponse)))

(fn GetCurrentHealth
  (return (Variables|/Game/OrcLaborContent/Blueprints/DamageSystem/RTS_BPC_DamageSystem.RTS_BPC_DamageSystem_C|GetHealth (Variables|Default|GetRTS_BPC_DamageSystem))))

(fn IsDead
  (return (Variables|/Game/OrcLaborContent/Blueprints/DamageSystem/RTS_BPC_DamageSystem.RTS_BPC_DamageSystem_C|GetIsDead (Variables|Default|GetRTS_BPC_DamageSystem))))

(fn Heal
  (params (AmountToHeal :type Float%20%28double-precision%29))
  (bind _newhealth (Default|Heal (Variables|Default|GetRTS_BPC_DamageSystem) AmountToHeal))
  (return _newhealth))

(fn TakeDamage
  (params (DamageInfo :type RTS%20S%20Damage%20Info%20Structure))
  (bind _wasdamaged (Default|TakeDamage (Variables|Default|GetRTS_BPC_DamageSystem) DamageInfo))
  (bind _health (CallFunction|GetCurrentHealth))
  (Variables|/Game/OrcLaborContent/Blueprints/UI/WB_UnitStatusBar.WB_UnitStatusBar_C|SetCurrentHealth (Variables|Default|GetUnitBarReference) _health)
  (Default|CallOnAttackFinished)
  (return _wasdamaged))

(fn GetMaxHealth
  (return (Variables|/Game/OrcLaborContent/Blueprints/DamageSystem/RTS_BPC_DamageSystem.RTS_BPC_DamageSystem_C|GetMaxHealth (Variables|Default|GetRTS_BPC_DamageSystem))))