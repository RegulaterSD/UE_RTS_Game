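; Player-controlled unit Blueprint that responds to move and selection commands, apparently for RTS-style control.
; Move commands stop the AI controller's current movement, then issue AI MoveTo toward the given location.
; Selection toggles a decal and adds or removes a per-unit icon widget, created at BeginPlay with a back-reference to the unit, in the player controller's selected-units area.
; Highlighting swaps the decal material.
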(event EventBeginPlay
  ;[1 1 1] Setup Selected Unit Widget
  (bind _returnvalue (UserInterface|CreateWidget "/Game/OrcLaborContent/Blueprints/UI/SelectedUnitWidget.SelectedUnitWidget_C"))
  (bind _output_get (Variables|Default|SetSelectedUnitWidget _returnvalue))
  (Variables|/Game/OrcLaborContent/Blueprints/UI/SelectedUnitWidget.SelectedUnitWidget_C|SetUnitReference _output_get self)
  (Appearance|SetBrushfromTexture (Variables|/Game/OrcLaborContent/Blueprints/UI/SelectedUnitWidget.SelectedUnitWidget_C|GetUnitIcon _returnvalue) (Variables|Default|GetUnitIcon) false))

(event EventHighlightUnit
  ;[1 1 1] Selection Highlight
  (Rendering|Components|Decal|SetDecalMaterial (Variables|Default|GetSelectionDecal) "/Game/OrcLaborContent/Assets/Cursor/Highlight_SelectedDecal.Highlight_SelectedDecal"))

(event EventUnHighlightUnit
  ;[1 1 1] Selection Highlight
  (Rendering|Components|Decal|SetDecalMaterial (Variables|Default|GetSelectionDecal) "/Game/OrcLaborContent/Assets/Cursor/SelectedDecal.SelectedDecal"))

(event EventSelectThis
  ;[1 1 1] Unit Selection
  (Development|PrintString "Selected")
  (Rendering|SetVisibility (Variables|Default|GetSelectionDecal) true false)
  (Class|RTSInterface|AddUnittoSelectedUnitsArea(Message) (Game|GetPlayerController 0) (Variables|Default|GetSelectedUnitWidget)))

(event EventDeselectThis
  ;[1 1 1] Unit Selection
  (Development|PrintString "Deselected")
  (Rendering|SetVisibility (Variables|Default|GetSelectionDecal) false false)
  (Widget|RemovefromParent (Variables|Default|GetSelectedUnitWidget)))

(event EventUnitMoveCommand
  (params (Location :type Vector :default "0, 0, 0"))
  (bind _self self)
  (bind _returnvalue (AI|GetAIController _self))
  ;[1 1 1] Player Unit Movment
  (AI|Navigation|StopMovement _returnvalue)
  (AI|AIMoveTo _returnvalue Location 0 -1.0 "Default" "Default" true true))

(fn ConstructionScript
  (|CallParentFunction))